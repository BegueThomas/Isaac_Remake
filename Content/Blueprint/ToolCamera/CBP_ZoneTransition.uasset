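; Camera zone trigger that, when the 2D player's capsule enters, moves the camera into the zone and starts its fight.
; It records overlapping doors, registers itself with the CameraManager, then a timeline lerps the camera to the zone's camera point.
; If the game is loaded and spawners overlap, BPI_Fight actors and GameMode get start messages; fight end notifies those actors and doors.
; Spline-follow, look-at and grid-move logic is disconnected.
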(event OnComponentBeginOverlap(Start)
  (params (OverlappedComponent :type Primitive%20Component%20Object%20Reference) (OtherActor :type Actor%20Object%20Reference) (OtherComp :type Primitive%20Component%20Object%20Reference) (OtherBodyIndex :type Integer) (bFromSweep :type Boolean) (SweepResult :type Hit%20Result%20Structure%20%28by%20ref%29))
  ;[0.15 0.15 0.15 0.5] Lorsque le joueur rentre dans la zone
  (if (== OtherComp (Variables|/Script/Engine.Character|GetCapsuleComponent (Variables|/Game/GameDesign/ThirdPerson/Blueprints/BP_ThirdPersonGameMode.BP_ThirdPersonGameMode_C|GetAs%20BP%20Player%202D (Variables|Default|GetRef_GameMode))))
    (CallFunction|StartMove)))

(event OnComponentEndOverlap(Start)
  (params (OverlappedComponent :type Primitive%20Component%20Object%20Reference) (OtherActor :type Actor%20Object%20Reference) (OtherComp :type Primitive%20Component%20Object%20Reference) (OtherBodyIndex :type Integer))
  ;[0.15 0.15 0.15 0.5] Lorsque le joueur sort de la zone
)

(event Custom|Start_Move
  (bind _ref_gamemode (Variables|Default|GetRef_GameMode))
  (bind _camera_manager (Variables|/Game/GameDesign/ThirdPerson/Blueprints/BP_ThirdPersonGameMode.BP_ThirdPersonGameMode_C|GetCamera_Manager _ref_gamemode))
  (for _array_element (Collision|GetOverlappingActors (Variables|Default|GetStart) "/Game/GameDesign/Blueprint/LD/Doors/BP_DoorTemplate.BP_DoorTemplate_C" :!class /Script/Engine.PrimitiveComponent)
    (bind _asbp_door_template (Utilities|Casting|CastToBP_DoorTemplate _array_element))
    (Utilities|Array|Add (Variables|Default|GetAffected_Doors) _asbp_door_template)
    (Variables|Default|SetStarting%20point (Transformation|GetActorLocation _camera_manager))
    (Variables|/Game/Blueprint/ToolCamera/BP_CameraManager.BP_CameraManager_C|SetZone _camera_manager self)
    (bind _float (Timeline|Transition_Camera PlayFromStart)
      (:Update
        (Transformation|SetActorLocation (Variables|/Game/GameDesign/ThirdPerson/Blueprints/BP_ThirdPersonGameMode.BP_ThirdPersonGameMode_C|GetCamera_Manager (Variables|Default|GetRef_GameMode)) (Math|Vector|Lerp(Vector) (Variables|Default|GetStarting%20point) (Transformation|GetWorldLocation (Variables|Default|GetBPS_LocationCamera)) _float) false false))
      (:Finished
        (CallFunction|FightStart)))))

(event Custom|RotateToPlayer
  ;[0.15 0.15 0.15 0.5] Camera se tourne vers le joueur
)

(event Custom|FollowPlayer
  ;[0.15 0.15 0.15 0.5] Caméra suis le joueur sur sa spline
)

(event Custom|Fight_Start
  (if (Variables|/Game/GameDesign/ThirdPerson/Blueprints/BP_ThirdPersonGameMode.BP_ThirdPersonGameMode_C|GetLoaded? (Variables|Default|GetRef_GameMode))
    (if (Utilities|Array|IsNotEmpty (Collision|GetOverlappingActors (Variables|Default|GetStart) "/Game/GameDesign/Blueprint/NPC/BP_MonsterSpawner.BP_MonsterSpawner_C" :!class /Script/Engine.PrimitiveComponent))
      (for _array_element (Collision|GetOverlappingActors (Variables|Default|GetStart) 0 :!class /Script/Engine.PrimitiveComponent)
        (if (Utilities|DoesObjectImplementInterface _array_element "/Game/GameDesign/BPI_Fight.BPI_Fight_C")
          (Class|BPIFight|FightStart(Message) _array_element)
          (Class|BPIFight|FightStart(Message) (Variables|Default|GetRef_GameMode)))))))

(event Custom|Fight_End
  (Utilities|FlowControl|Sequence
    (:then_0
      (for _array_element (Collision|GetOverlappingActors (Variables|Default|GetStart) 0 :!class /Script/Engine.PrimitiveComponent)
        (if (Utilities|DoesObjectImplementInterface _array_element "/Game/GameDesign/BPI_Fight.BPI_Fight_C")
          (Class|BPIFight|FightEnd(Message) _array_element))))
    (:then_1
      (for _array_element_2 (Variables|Default|GetAffected_Doors)
        (Class|BPIFight|FightEnd(Message) _array_element_2)))))

(event EventBeginPlay
  (bind _asbp_third_person_game_mode (Utilities|Casting|CastToBP_ThirdPersonGameMode (Game|GetGameMode)))
  (Variables|Default|SetRef_GameMode _asbp_third_person_game_mode))

(event Collision|EventActorBeginOverlap
  (params (OtherActor :type Actor%20Object%20Reference)))

(event EventActivate
  ;[0.15 0.15 0.15 0.5] active la cinematique de l'acteur
)

(event EventTick
  (params (DeltaSeconds :type Float%20%28single-precision%29)))

(fn ConstructionScript)

(fn GetClosestPosonSpline
  (params (Location :type Vector) (Speed :type Float%20%28double-precision%29))
  (bind _spline (Variables|Default|GetSpline))
  (if (< (LocalVariables|GetCheckLength) (Spline|GetSplineLength _spline)) :!label _label
    (if (> (LocalVariables|GetClosestDistance) (Math|Vector|Distance(Vector) (Spline|GetLocationatDistanceAlongSpline _spline (LocalVariables|GetCheckLength) "World") Location))
      (LocalVariables|SetClosestDistance (Math|Vector|Distance(Vector) (Spline|GetLocationatDistanceAlongSpline _spline (LocalVariables|GetCheckLength) "World") Location))
      (LocalVariables|SetLenghtAtClosest (LocalVariables|GetCheckLength)))
    (LocalVariables|SetCheckLength (+ (LocalVariables|GetCheckLength) 1.0))
    (goto _label)
    (else
      (return (LocalVariables|GetLenghtAtClosest)))))