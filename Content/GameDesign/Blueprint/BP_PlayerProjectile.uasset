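; Player projectile Blueprint that takes its pierce, speed and lifetime from the player's ProjectileInfo stats.
; On BeginPlay it finds BP_Player2D at player index 0, records it as Creator, copies the stats, then hands off to the parent BeginPlay.
; The Distance stat is used directly as the actor's life span.
; Update_Stat_Proj re-reads the same stats from the cached player reference.
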(event Custom|Update_Stat_Proj
  (bind _player_ref (Variables|Default|GetPlayer_Ref))
  (bind _projectile_info (Variables|/Game/GameDesign/ThirdPerson/Blueprints/BP_Player2D.BP_Player2D_C|GetProjectile_Info _player_ref))
  (bind (_modf_fire_rate _pierce _damage _proj_speed _distance) (Utilities|Struct|BreakST_Projectile _projectile_info))
  (Variables|Default|Setpierce _pierce)
  (Variables|Default|SetSpeed _proj_speed)
  (Actor|SetLifeSpan _distance))

(event EventBeginPlay
  (bind _asbp_player_2d (Utilities|Casting|CastToBP_Player2D (Game|Player|GetPlayerPawn 0)))
  (bind _output_get (Variables|Default|SetPlayer_Ref _asbp_player_2d))
  (Variables|Default|SetCreator _output_get)
  (bind _output_get_2 (Variables|Default|SetProjectile_Stats (Variables|/Game/GameDesign/ThirdPerson/Blueprints/BP_Player2D.BP_Player2D_C|GetProjectile_Info (Variables|Default|GetPlayer_Ref))))
  (Variables|Default|Setpierce (.Pierce (Utilities|Struct|BreakST_Projectile _output_get_2)))
  (Variables|Default|SetSpeed (.Proj_Speed (Utilities|Struct|BreakST_Projectile _output_get_2)))
  (Actor|SetLifeSpan (.Distance (Utilities|Struct|BreakST_Projectile _output_get_2)))
  (|CallParentFunction))

(event Collision|EventActorBeginOverlap
  (params (OtherActor :type Actor%20Object%20Reference))
  (|CallParentFunction OtherActor) ; This node is disabled and will not be called.\nDrag off pins to build functionality.
)

(event EventTick
  (params (DeltaSeconds :type Float%20%28single-precision%29))
  (|CallParentFunction DeltaSeconds) ; This node is disabled and will not be called.\nDrag off pins to build functionality.
)

(fn ConstructionScript)