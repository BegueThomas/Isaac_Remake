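; Data-table-driven projectile that damages actors its sphere overlaps, with pierce, speed, damage and lifespan read from its row at construction.
; Tick advances it forward unless a short line trace is blocked, storing a base point.
; A looping timeline, using the row's curve, offsets that point sideways to shape the flight path.
; Each overlap spends pierce; once below zero it spawns VFX, plays a sound and destroys itself.
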(event OnComponentBeginOverlap(Sphere)
  (params (OverlappedComponent :type Primitive%20Component%20Object%20Reference) (OtherActor :type Actor%20Object%20Reference) (OtherComp :type Primitive%20Component%20Object%20Reference) (OtherBodyIndex :type Integer) (bFromSweep :type Boolean) (SweepResult :type Hit%20Result%20Structure%20%28by%20ref%29))
  (CallFunction|Damage OtherActor))

(event OnComponentBeginOverlap(PaperSprite)
  (params (OverlappedComponent :type Primitive%20Component%20Object%20Reference) (OtherActor :type Actor%20Object%20Reference) (OtherComp :type Primitive%20Component%20Object%20Reference) (OtherBodyIndex :type Integer) (bFromSweep :type Boolean) (SweepResult :type Hit%20Result%20Structure%20%28by%20ref%29)))

(event Custom|Restart
  (Components|Timeline|PlayfromStart (Variables|Default|GetMove_Curve)))

(event Collision|EventActorBeginOverlap
  (params (OtherActor :type Actor%20Object%20Reference)))

(event EventTick
  (params (DeltaSeconds :type Float%20%28single-precision%29))
  (Variables|Default|SetDelta%20Seconds DeltaSeconds)
  (bind _returnvalue1 (CallFunction|TryMove (Transformation|GetActorLocation) (Math|Vector|GetForwardVector (Transformation|GetActorRotation)) (* (Variables|Default|GetSpeed) (Variables|Default|GetDelta%20Seconds)) "Blcoked" 1e+01))
  (Variables|Default|SetStart_Point _returnvalue1))

(event EventBeginPlay
  (bind _projectile_stats (Variables|Default|GetProjectile_Stats))
  (Audio|PlaySound2D "/Game/Sound/shoot-f.shoot-f" 1.0 1.0 0.0 0 0)
  (Variables|Default|SetSide_Vector (Transformation|GetActorRightVector))
  (Development|PrintString (Utilities|GetDisplayName (.curve _projectile_stats)))
  (Class|TimelineComponent|SetFloatCurve (Variables|Default|GetMove_Curve) (.curve _projectile_stats) "Float")
  (bind _float (Timeline|Move_Curve Play)
    (:Update
      (Transformation|SetActorLocation (+ (Variables|Default|GetStart_Point) (* (* _float 5.0) (Variables|Default|GetSide_Vector))) false false))
    (:Finished
      (CallFunction|Restart))))

(fn ConstructionScript
  (bind _data_row (Variables|Default|GetData_Row))
  (bind _returnvalue (Utilities|GetDataTableRow (.datatable _data_row) (.rowname _data_row))
    (:then
      (bind _output_get (Variables|Default|SetProjectile_Stats _returnvalue))
      (Variables|Default|Setpierce (.Pierce (Utilities|Struct|BreakST_Projectile _output_get)))
      (Variables|Default|SetSpeed (.Proj_Speed (Utilities|Struct|BreakST_Projectile _output_get)))
      (Actor|SetLifeSpan (.Distance (Utilities|Struct|BreakST_Projectile _output_get))))))

(fn TryMove
  (params (Start :type Vector) (Direction :type Vector) (MovementSpeed :type Float%20%28double-precision%29) (Message :type String) (Distance_Trace :type Float%20%28double-precision%29))
  (bind _returnvalue (Transformation|GetActorLocation))
  (bind _returnvalue_2 (* Direction MovementSpeed))
  (bind _returnvalue_3 (+ _returnvalue _returnvalue_2))
  (bind (_outhit _returnvalue_4) (Collision|LineTraceByChannel Start (+ Start (* Direction Distance_Trace)) "TraceTypeQuery1" false 0 "None" true "(R=1.000000,G=0.000000,B=0.000000,A=1.000000)" "(R=0.000000,G=1.000000,B=0.000000,A=1.000000)" 0.2))
  (if _returnvalue_4
    _
    (else
      (Transformation|SetActorLocation _returnvalue_3 true false)))
  (return _outhit _returnvalue_4 _returnvalue_3))

(fn Damage
  (params (Target :type Actor%20Object%20Reference))
  (CallFunction|AddTargetHealth Target (.Damage (Utilities|Struct|BreakST_Projectile (Variables|Default|GetProjectile_Stats))))
  (bind _output_get (Variables|Default|Setpierce (- (Variables|Default|Getpierce) 1.0)))
  (if (< _output_get 0.0)
    (Game|SpawnActorfromClass (Variables|Default|GetVFX) (Transformation|GetActorTransform) "Undefined" "MultiplyWithRoot" 0 0)
    (Audio|PlaySound2D "/Game/Sound/hurt-a.hurt-a" 1.0 1.0 0.0 0 0)
    (Actor|DestroyActor)))