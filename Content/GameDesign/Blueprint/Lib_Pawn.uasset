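; Blueprint function library of shared pawn helpers for changing a target's health and the player's coins.
; AddTargetHealth adds a signed amount to the player, a breakable or a monster via casts, triggering Death, or DestroyActor for breakables, at zero or below.
; Player damage reactions fire only on negative amounts, while breakable Damaged and monster Stun fire on any change.
; AddTargetCoin increases the coin count only when the target is the player pawn.
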(fn AddTargetHealth
  (params (Target :type Actor%20Object%20Reference) (Amount :type Float%20%28double-precision%29))
  (if (== Target (Game|Player|GetPlayerPawn 0))
    (bind _asbp_player_2d (Utilities|Casting|CastToBP_Player2D Target))
    (if (< Amount 0.0)
      (Default|Damaged _asbp_player_2d)
      (Audio|PlaySound2D 0 "/Game/Sound/hurt-a_Cue.hurt-a_Cue" 1.0 1.0 0.0 0 0))
    (bind _output_get (Variables|/Game/GameDesign/ThirdPerson/Blueprints/BP_Player2D.BP_Player2D_C|SetCurrent_Health _asbp_player_2d (+ (Variables|/Game/GameDesign/ThirdPerson/Blueprints/BP_Player2D.BP_Player2D_C|GetCurrent_Health _asbp_player_2d) Amount)))
    (if (<= _output_get 0.0)
      (Default|Death _asbp_player_2d))
    (else
      (bind _asbp_breakable (Utilities|Casting|CastToBP_Breakable Target)
        (:then
          (Default|Damaged _asbp_breakable)
          (bind _output_get_2 (Variables|/Game/GameDesign/Blueprint/BP_Breakable.BP_Breakable_C|SetHealth _asbp_breakable (+ (Variables|/Game/GameDesign/Blueprint/BP_Breakable.BP_Breakable_C|GetHealth _asbp_breakable) Amount)))
          (if (<= _output_get_2 0.0)
            (Actor|DestroyActor _asbp_breakable)))
        (:CastFailed
          (bind _asbp_monster_template (Utilities|Casting|CastToBP_MonsterTemplate Target))
          (Default|Stun _asbp_monster_template)
          (Audio|PlaySound2D 0 "/Game/Sound/hurt-a_Cue.hurt-a_Cue" 1.0 1.0 0.0 0 0)
          (bind _output_get_3 (Variables|/Game/GameDesign/Blueprint/NPC/BP_MonsterTemplate.BP_MonsterTemplate_C|SetCurrent_Health _asbp_monster_template (+ (Variables|/Game/GameDesign/Blueprint/NPC/BP_MonsterTemplate.BP_MonsterTemplate_C|GetCurrent_Health _asbp_monster_template) Amount)))
          (if (<= _output_get_3 0.0)
            (Default|Death _asbp_monster_template)))))))

(fn AddTargetCoin
  (params (Target :type Actor%20Object%20Reference) (Amount :type Float%20%28double-precision%29))
  (if (== Target (Game|Player|GetPlayerPawn 0))
    (bind _asbp_player_2d (Utilities|Casting|CastToBP_Player2D Target))
    (Variables|/Game/GameDesign/ThirdPerson/Blueprints/BP_Player2D.BP_Player2D_C|SetCoin _asbp_player_2d (+ (Variables|/Game/GameDesign/ThirdPerson/Blueprints/BP_Player2D.BP_Player2D_C|GetCoin _asbp_player_2d) Amount))
    (return false)))