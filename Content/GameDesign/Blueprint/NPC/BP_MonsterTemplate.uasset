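; Template 2D monster that chases the player and attacks in melee or at range, configured by pawn and projectile data table rows.
; Tick steps toward the player via line-traced moves that trigger melee on hit, and ranged types fire projectiles, both attacks gated by timeline cooldowns.
; Stun briefly halts movement with a red flash, overlapping monsters push apart, and death notifies the GameMode before destroying the actor.
; PCG spline-following logic is present but unconnected.
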(event OnComponentBeginOverlap(CapsuleComponent)
  (params (OverlappedComponent :type Primitive%20Component%20Object%20Reference) (OtherActor :type Actor%20Object%20Reference) (OtherComp :type Primitive%20Component%20Object%20Reference) (OtherBodyIndex :type Integer) (bFromSweep :type Boolean) (SweepResult :type Hit%20Result%20Structure%20%28by%20ref%29))
  (bind _asbp_monster_template (Utilities|Casting|CastToBP_MonsterTemplate OtherActor))
  (CallFunction|Push _asbp_monster_template 4.0))

(event Custom|MoveTowardsPlayer
  (bind _returnvalue (Transformation|GetActorLocation))
  (bind _pawn_info (Variables|Default|GetPawn_Info))
  (if (not (.static? _pawn_info))
    (if (not (Variables|Default|GetStun?))
      (bind (_outhit _returnvalue_2) (CallFunction|TryMove _returnvalue (Math|Vector|GetUnitDirection(Vector) _returnvalue (Variables|Default|GetPlayer_Pos)) (* (.move_speed _pawn_info) (Variables|Default|GetDelta%20Seconds)) "Blcoked" (.range_melee _pawn_info)))
      (if _returnvalue_2
        (CallFunction|MeleeEvent (.HitActor (Collision|BreakHitResult _outhit)))))))

(event Custom|GetPlayerPosition
  (Variables|Default|SetPlayer_Pos (Transformation|GetActorLocation (Variables|Default|GetPlayer_Ref))))

(event Custom|Melee_Event
  (params (Target :type Actor%20Object%20Reference))
  (bind _pawn_info (Variables|Default|GetPawn_Info))
  (if (.attackmelle? _pawn_info)
    (if (not (Variables|Default|GetAttack?))
      (Variables|Default|SetAttack? true)
      (CallFunction|AddTargetHealth Target (.damage _pawn_info))
      (Components|Timeline|SetTimelineLength (Variables|Default|GetCoolDown) (* (Variables|Default|GetAttack_Delay) (.att_speed _pawn_info)))
      (Timeline|CoolDown PlayFromStart
        (:Finished
          (Variables|Default|SetAttack? false))))))

(event Custom|Death
  (bind _sprite (Variables|Default|GetSprite))
  (if (not (Variables|Default|GetDead))
    (Variables|Default|SetDead true)
    (Default|EnnemyDeath (Variables|Default|GetGameMod_Ref))
    (Sprite|SetFlipbook _sprite (Variables|Default|GetDeathAnim))
    (Components|Timeline|SetLooping _sprite false)
    (Game|SpawnActorfromClass "/Game/GameDesign/Blueprint/VFX/BP_VFX_Spawn.BP_VFX_Spawn_C" (Transformation|GetActorTransform) "Undefined" "MultiplyWithRoot" 0 0)
    (Utilities|FlowControl|Delay 0.2)
    (Actor|DestroyActor)))

(event Custom|Stun
  (Sprite|SetSpriteColor (Variables|Default|GetSprite) "(R=1.000000,G=0.006070,B=0.000000,A=1.000000)")
  (Variables|Default|SetStun? true)
  (Utilities|FlowControl|Delay 0.2)
  (Variables|Default|SetStun? false)
  (Sprite|SetSpriteColor (Variables|Default|GetSprite) "(R=1.000000,G=1.000000,B=1.000000,A=1.000000)"))

(event Custom|Shoot_Event
  (bind _shootdirection (Variables|Default|GetShootDirection))
  (bind _returnvalue (Transformation|GetWorldTransform _shootdirection))
  ;[0.15 0.15 0.15 0.5] Set la direction du tirs
  (Transformation|SetWorldRotation (Variables|Default|GetShootDirection) (Math|Rotator|FindLookatRotation (Transformation|GetWorldLocation (Variables|Default|GetShootDirection)) (Transformation|GetActorLocation (Game|Player|GetPlayerPawn 0))) false false)
  (if (not (Variables|Default|GetShooting?))
    (Variables|Default|SetShooting? true)
    (bind _returnvalue_2 (Game|SpawnActorfromClass "/Game/GameDesign/Blueprint/BP_Projectile_Monster.BP_Projectile_Monster_C" (Math|Transform|MakeTransform (+ (.location _returnvalue) (* (Math|Vector|GetForwardVector (.rotation _returnvalue)) 5e+01)) (.rotation _returnvalue) "1.000000,1.000000,1.000000") "Undefined" "MultiplyWithRoot" 0 0))
    (Variables|/Game/GameDesign/Blueprint/BP_Projectile.BP_Projectile_C|SetCreator _returnvalue_2 self)
    (Components|Timeline|SetTimelineLength (Variables|Default|GetCD_Shoot) (* (Variables|Default|GetProj_Delay) (.modf_fire_rate (Variables|Default|GetProjectile_Info))))
    (bind _float (Timeline|CD_Shoot PlayFromStart)
      (:Update
        (Transformation|SetRelativeScale3D (Variables|Default|GetProjectile_Sprite) (Math|Vector|Lerp(Vector) "0, 0, 0" "1.000000,1.000000,1.000000" _float)))
      (:Finished
        (Variables|Default|SetShooting? false)))))

(event EventBeginPlay
  (bind _dt_rowprojectile (Variables|Default|GetDT_RowProjectile))
  (bind _dt_rowpawnstat (Variables|Default|GetDT_RowPawnStat))
  (bind _asbp_third_person_game_mode (Utilities|Casting|CastToBP_ThirdPersonGameMode (Game|GetGameMode)))
  (Variables|Default|SetGameMod_Ref _asbp_third_person_game_mode)
  (bind _asbp_player_2d (Utilities|Casting|CastToBP_Player2D (Game|Player|GetPlayerPawn 0)))
  (Variables|Default|SetPlayer_Ref _asbp_player_2d)
  (bind _returnvalue (Utilities|GetDataTableRow (.datatable _dt_rowprojectile) (.rowname _dt_rowprojectile))
    (:then
      (Variables|Default|SetProjectile_Info _returnvalue)
      (bind _returnvalue_2 (Utilities|GetDataTableRow (.datatable _dt_rowpawnstat) (.rowname _dt_rowpawnstat))
        (:then
          (Variables|Default|SetPawn_Info _returnvalue_2)
          (Variables|Default|SetCurrent_Health (.Max_Life (Utilities|Struct|BreakST_PawnStat _returnvalue_2))))))))

(event Collision|EventActorBeginOverlap
  (params (OtherActor :type Actor%20Object%20Reference)))

(event EventTick
  (params (DeltaSeconds :type Float%20%28single-precision%29))
  (Variables|Default|SetDelta%20Seconds DeltaSeconds)
  (if (not (Variables|Default|GetDead))
    (CallFunction|GetPlayerPosition)
    (CallFunction|MoveTowardsPlayer)
    (if (.attack_range? (Variables|Default|GetPawn_Info))
      (CallFunction|ShootEvent))))

(fn ConstructionScript)

(fn TryMove
  (params (Start :type Vector) (Direction :type Vector) (MovementSpeed :type Float%20%28double-precision%29) (Message :type String) (Distance_Trace :type Float%20%28double-precision%29))
  (bind (_outhit _returnvalue) (Collision|LineTraceByChannel Start (+ Start (* Direction Distance_Trace)) "TraceTypeQuery1" false 0 "None" true "(R=0.019157,G=1.000000,B=0.000000,A=1.000000)" "(R=1.000000,G=0.018427,B=0.000073,A=1.000000)" 0.2))
  (if _returnvalue
    (Development|PrintString Message false false)
    (else
      (Transformation|SetActorLocation (+ (Transformation|GetActorLocation) (* Direction MovementSpeed)) true false)))
  (return _outhit _returnvalue))

(fn Melee
  (params (Target :type Actor%20Object%20Reference))
  (bind _pawn_info (Variables|Default|GetPawn_Info))
  (if (.attackmelle? _pawn_info)
    (CallFunction|AddTargetHealth Target (.damage _pawn_info))))

(fn Push
  (params (Push_Source :type Actor%20Object%20Reference) (Push_MoveSpeed :type Float%20%28double-precision%29))
  (bind _returnvalue (Transformation|GetActorLocation))
  (bind _arrow_push (Variables|Default|GetArrow_Push))
  (Transformation|SetWorldRotation _arrow_push (Math|Rotator|MakeRotator 0.0 0.0 (.yaw (Math|Rotator|FindLookatRotation (Transformation|GetActorLocation Push_Source) _returnvalue))) false false)
  (CallFunction|TryMove _returnvalue (Math|Vector|GetForwardVector (Transformation|GetWorldRotation _arrow_push)) Push_MoveSpeed "Blcoked" 1e+01))