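; BP_Monster_BOSS is a flipbook-sprite boss NPC whose death ends play by pausing the game behind a UI screen.
; Its only active logic is a one-shot Death event that notifies the game mode, plays the non-looping death animation and spawns the BP_VFX_Spawn effect.
; After the animation and a short delay, it shows UI_Death1, switches to UI-only input with a mouse cursor, and pauses the game.
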(event EventBeginPlay
  (|CallParentFunction) ; This node is disabled and will not be called.\nDrag off pins to build functionality.
)

(event Collision|EventActorBeginOverlap
  (params (OtherActor :type Actor%20Object%20Reference))
  (|CallParentFunction OtherActor) ; This node is disabled and will not be called.\nDrag off pins to build functionality.
)

(event EventTick
  (params (DeltaSeconds :type Float%20%28single-precision%29))
  (|CallParentFunction DeltaSeconds) ; This node is disabled and will not be called.\nDrag off pins to build functionality.
)

(event EventDeath
  (bind _returnvalue (Game|GetPlayerController 0))
  (bind _sprite (Variables|Default|GetSprite))
  (if (not (Variables|Default|GetDead))
    (Variables|Default|SetDead true)
    (Default|EnnemyDeath (Variables|Default|GetGameMod_Ref))
    (Sprite|SetFlipbook _sprite (Variables|Default|GetDeathAnim))
    (Components|Timeline|SetLooping _sprite false)
    (Game|SpawnActorfromClass "/Game/GameDesign/Blueprint/VFX/BP_VFX_Spawn.BP_VFX_Spawn_C" (Transformation|GetActorTransform) "Undefined" "MultiplyWithRoot" 0 0)
    (Utilities|FlowControl|Delay (+ (Class|PaperFlipbookComponent|GetFlipbookLength _sprite) 0.5))
    (bind _returnvalue_2 (UserInterface|CreateWidget "/Game/UI/UI_Death1.UI_Death1_C"))
    (UserInterface|Viewport|AddtoViewport _returnvalue_2 2)
    (Input|SetInputModeUIOnly _returnvalue 0 "DoNotLock" false)
    (Variables|/Script/Engine.PlayerController|SetbShowMouseCursor _returnvalue true)
    (Game|SetGamePaused true)))

(fn ConstructionScript
  (|CallParentFunction))