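; BP_Chest is a pickup chest that releases random loot the first time it is triggered.
; Every PickUpEvent calls Push with the triggering target as source and swaps the Paper2D sprite.
; An Opened flag limits loot to one burst of three to five random LootPool items, spawned at the chest.
; Each item eases toward a randomly scaled negative right vector, used without adding the chest's location.
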(event EventBeginPlay
  (|CallParentFunction) ; This node is disabled and will not be called.\nDrag off pins to build functionality.
)

(event Collision|EventActorBeginOverlap
  (params (OtherActor :type Actor%20Object%20Reference))
  (|CallParentFunction OtherActor) ; This node is disabled and will not be called.\nDrag off pins to build functionality.
)

(event EventTick
  (params (DeltaSeconds :type Float%20%28single-precision%29))
  (|CallParentFunction DeltaSeconds) ; This node is disabled and will not be called.\nDrag off pins to build functionality.
)

(event EventPickUpEvent
  (params (Target :type Actor%20Object%20Reference))
  (CallFunction|Push Target 4e+01)
  (Rendering|Components|Sprite|SetSprite (Variables|Default|GetPaperSprite) "/Game/PaperAssets/Tilemap/Sprites_TileMap/tilemap_Sprite_217.tilemap_Sprite_217")
  (if (not (Variables|Default|GetOpened?))
    (Variables|Default|SetOpened? true)
    (for _index (range 0 (Math|Random|RandomIntegerinRange 3 5))
      (bind _returnvalue (Game|SpawnActorfromClass (.OutItem (Utilities|Array|Random (Variables|Default|GetLoot_Pool))) (Math|Transform|MakeTransform (Transformation|GetActorLocation) "0, 0, 0" "1.000000,1.000000,1.000000") "AlwaysSpawn" "MultiplyWithRoot" 0 0))
      (Components|MoveComponentTo (Variables|/Script/Engine.Actor|GetRootComponent _returnvalue) (* (Transformation|GetActorRightVector) (Math|Random|RandomFloatinRange -1e+02 -2e+02)) "0, 0, 0" true true 0.2 false))))

(fn ConstructionScript
  (|CallParentFunction))