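; BP_PickUp is a pickup actor with an empty pickup event, which caches the game mode on BeginPlay.
; When the player pawn overlaps its box, it fires the pickup event and plays a coin sound.
; Any other overlapping actor pushes it away along an arrow turned by look-at yaw, by a random amount.
; A short line trace must find no obstruction before an eased MoveComponentTo slides the root.
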(event OnComponentBeginOverlap(Box)
  (params (OverlappedComponent :type Primitive%20Component%20Object%20Reference) (OtherActor :type Actor%20Object%20Reference) (OtherComp :type Primitive%20Component%20Object%20Reference) (OtherBodyIndex :type Integer) (bFromSweep :type Boolean) (SweepResult :type Hit%20Result%20Structure%20%28by%20ref%29))
  (if (== OtherActor (Game|Player|GetPlayerPawn 0))
    (CallFunction|PickUpEvent OtherActor)
    (Audio|PlaySound2D "/Game/Sound/coin-b_Cue.coin-b_Cue" 1.0 1.0 0.0 0 0)
    (else
      (CallFunction|Push OtherActor (Math|Random|RandomFloatinRange 5.0 1e+01)))))

(event Custom|PickUp_Event
  (params (Target :type Actor%20Object%20Reference)))

(event Custom|MoveTo
  (params (TargetRelativeLocation :type Vector) (OverTime :type Float%20%28double-precision%29))
  (Components|MoveComponentTo (Variables|Default|GetDefaultSceneRoot) TargetRelativeLocation "0, 0, 0" true true OverTime false))

(event EventBeginPlay
  (bind _asbp_third_person_game_mode (Utilities|Casting|CastToBP_ThirdPersonGameMode (Game|GetGameMode)))
  (Variables|Default|SetGameModeRef _asbp_third_person_game_mode))

(event Collision|EventActorBeginOverlap
  (params (OtherActor :type Actor%20Object%20Reference)))

(event EventTick
  (params (DeltaSeconds :type Float%20%28single-precision%29)))

(fn ConstructionScript)

(fn TryMove
  (params (Start :type Vector) (Direction :type Vector) (MovementSpeed :type Float%20%28double-precision%29) (Message :type String) (Distance_Trace :type Float%20%28double-precision%29))
  (bind (_outhit _returnvalue) (Collision|LineTraceByChannel Start (+ Start (* Direction Distance_Trace)) "TraceTypeQuery1" false 0 "None" true "(R=0.019157,G=1.000000,B=0.000000,A=1.000000)" "(R=1.000000,G=0.018427,B=0.000073,A=1.000000)" 0.2))
  (if (not _returnvalue)
    (CallFunction|Moveto (+ (Transformation|GetActorLocation) (* Direction MovementSpeed)) 0.2)
    (return _outhit _returnvalue)))

(fn Push
  (params (Push_Source :type Actor%20Object%20Reference) (Push_MoveSpeed :type Float%20%28double-precision%29))
  (bind _returnvalue (Transformation|GetActorLocation))
  (bind _arrow (Variables|Default|GetArrow))
  (Transformation|SetWorldRotation _arrow (Math|Rotator|MakeRotator 0.0 0.0 (.yaw (Math|Rotator|FindLookatRotation (Transformation|GetActorLocation Push_Source) _returnvalue))) false false)
  (CallFunction|TryMove _returnvalue (Math|Vector|GetForwardVector (Transformation|GetWorldRotation _arrow)) Push_MoveSpeed "Blcoked" 1e+01))