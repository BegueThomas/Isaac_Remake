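; BP_PickUp_Item is a stat pickup that modifies the 2D player's PawnInfo when collected, then destroys itself.
; PickUpEvent adds the item's AddStat max life and move speed to the player's values, reached through GameModeRef, using VerifyAddStats to floor each sum at zero.
; The rebuilt struct sets all other fields to fixed literals instead of copying their current values.
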(event EventBeginPlay
  (|CallParentFunction) ; This node is disabled and will not be called.\nDrag off pins to build functionality.
)

(event Collision|EventActorBeginOverlap
  (params (OtherActor :type Actor%20Object%20Reference))
  (|CallParentFunction OtherActor) ; This node is disabled and will not be called.\nDrag off pins to build functionality.
)

(event EventTick
  (params (DeltaSeconds :type Float%20%28single-precision%29))
  (|CallParentFunction DeltaSeconds) ; This node is disabled and will not be called.\nDrag off pins to build functionality.
)

(event EventPickUpEvent
  (params (Target :type Actor%20Object%20Reference))
  (bind _gamemoderef (Variables|Default|GetGameModeRef))
  (bind _add_stat (Variables|Default|GetAdd_Stat))
  (bind _as_bp_player_2d (Variables|/Game/GameDesign/ThirdPerson/Blueprints/BP_ThirdPersonGameMode.BP_ThirdPersonGameMode_C|GetAs%20BP%20Player%202D _gamemoderef))
  (Variables|/Game/GameDesign/ThirdPerson/Blueprints/BP_Player2D.BP_Player2D_C|SetPawn_Info _as_bp_player_2d (Utilities|Struct|MakeST_PawnStat (CallFunction|VerifyAddStats (.max_life (Variables|/Game/GameDesign/ThirdPerson/Blueprints/BP_Player2D.BP_Player2D_C|GetPawn_Info _as_bp_player_2d)) (.max_life _add_stat)) (CallFunction|VerifyAddStats (.move_speed (Variables|/Game/GameDesign/ThirdPerson/Blueprints/BP_Player2D.BP_Player2D_C|GetPawn_Info _as_bp_player_2d)) (.move_speed _add_stat)) 1.0 1.0 8e+01 true false false false))
  (Actor|DestroyActor))

(fn ConstructionScript
  (|CallParentFunction))

(fn VerifyAddStats
  (params (A :type Float%20%28double-precision%29) (B :type Float%20%28double-precision%29))
  (bind _returnvalue (+ A B))
  (if (<= _returnvalue 0.0)
    (return 0.0)
    (else
      (return _returnvalue))))