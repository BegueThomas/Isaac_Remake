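; Shop pickup actor that selects a random item from a shop data table.
; On BeginPlay it picks a random row of DTSHOP and stores it as ItemInfo.
; PickUpEvent only passes Price to AddTargetCoin on the target; it does not grant the item.
; The node that spawns the ItemInfo item class is unconnected, and GivenItem is unused.
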(event EventBeginPlay
  (bind _dt_shop (Variables|Default|GetDT_SHOP))
  (|CallParentFunction)
  (bind _outrownames (DataTable|GetDataTableRowNames (.datatable _dt_shop)))
  (bind _returnvalue (Utilities|GetDataTableRow (.datatable _dt_shop) (.OutItem (Utilities|Array|Random _outrownames)))
    (:then
      (Variables|Default|SetItem_Info _returnvalue))))

(event Collision|EventActorBeginOverlap
  (params (OtherActor :type Actor%20Object%20Reference))
  (|CallParentFunction OtherActor) ; This node is disabled and will not be called.\nDrag off pins to build functionality.
)

(event EventTick
  (params (DeltaSeconds :type Float%20%28single-precision%29))
  (|CallParentFunction DeltaSeconds) ; This node is disabled and will not be called.\nDrag off pins to build functionality.
)

(event EventPickUpEvent
  (params (Target :type Actor%20Object%20Reference))
  (CallFunction|AddTargetCoin Target (Variables|Default|GetPrice)))

(fn ConstructionScript
  (|CallParentFunction))