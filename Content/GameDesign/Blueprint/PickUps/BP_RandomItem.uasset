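; BP_RandomItem is a pickup placeholder actor that spawns a random item at its own location when play begins.
; On BeginPlay it picks a random class from its LootPool array and spawns it, ignoring collisions.
; The placeholder does not destroy itself afterwards, and its construction script only calls the parent.
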(event EventBeginPlay
  (|CallParentFunction)
  (Game|SpawnActorfromClass (.OutItem (Utilities|Array|Random (Variables|Default|GetLoot_Pool))) (Math|Transform|MakeTransform (Transformation|GetActorLocation) "0, 0, 0" "1.000000,1.000000,1.000000") "AlwaysSpawn" "MultiplyWithRoot" 0 0))

(event Collision|EventActorBeginOverlap
  (params (OtherActor :type Actor%20Object%20Reference))
  (|CallParentFunction OtherActor) ; This node is disabled and will not be called.\nDrag off pins to build functionality.
)

(event EventTick
  (params (DeltaSeconds :type Float%20%28single-precision%29))
  (|CallParentFunction DeltaSeconds) ; This node is disabled and will not be called.\nDrag off pins to build functionality.
)

(fn ConstructionScript
  (|CallParentFunction))