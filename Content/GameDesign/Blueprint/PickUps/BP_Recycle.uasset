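; BP_Recycle is a single-use recycler pickup that trades a random item from the player's inventory for a heart container.
; PickUpEvent calls Push and, if unused with items available, triggers Nullify to subtract item stats from ProjectileInfo through the zero-clamping VerifyAddStats helper.
; Nullify removes an item, refreshes the widget, spawns the heart and swaps the sprite.
; Random is re-evaluated between steps, so the subtracted and removed items can differ.
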(event Custom|Nullify
  (bind _gamemoderef (Variables|Default|GetGameModeRef))
  (bind _gamemoderef_2 (Variables|Default|GetGameModeRef))
  (bind _as_bp_player_2d (Variables|/Game/GameDesign/ThirdPerson/Blueprints/BP_ThirdPersonGameMode.BP_ThirdPersonGameMode_C|GetAs%20BP%20Player%202D _gamemoderef))
  (bind _as_bp_player_2d_2 (Variables|/Game/GameDesign/ThirdPerson/Blueprints/BP_ThirdPersonGameMode.BP_ThirdPersonGameMode_C|GetAs%20BP%20Player%202D _gamemoderef_2))
  (bind _item_list (Variables|/Game/GameDesign/ThirdPerson/Blueprints/BP_Player2D.BP_Player2D_C|GetItem_List _as_bp_player_2d_2))
  (bind _outitem (Utilities|Array|Random _item_list))
  (bind (_item _count _sprite _object _ref_addstat) (Utilities|Struct|BreakST_ItemList _outitem))
  (bind (_modf_fire_rate _pierce _damage _proj_speed _distance) (Utilities|Struct|BreakST_Projectile _ref_addstat))
  (for _index (range 1 (Math|Float|Truncate _count))
    (Variables|/Game/GameDesign/ThirdPerson/Blueprints/BP_Player2D.BP_Player2D_C|SetProjectile_Info _as_bp_player_2d (Utilities|Struct|MakeST_Projectile (CallFunction|VerifyAddStats (.modf_fire_rate (Variables|/Game/GameDesign/ThirdPerson/Blueprints/BP_Player2D.BP_Player2D_C|GetProjectile_Info _as_bp_player_2d)) (* _modf_fire_rate -1.0)) (CallFunction|VerifyAddStats (.pierce (Variables|/Game/GameDesign/ThirdPerson/Blueprints/BP_Player2D.BP_Player2D_C|GetProjectile_Info _as_bp_player_2d)) (* _pierce -1.0)) (* (CallFunction|VerifyAddStats (* (.damage (Variables|/Game/GameDesign/ThirdPerson/Blueprints/BP_Player2D.BP_Player2D_C|GetProjectile_Info _as_bp_player_2d)) -1.0) _damage) -1.0) (CallFunction|VerifyAddStats (.proj_speed (Variables|/Game/GameDesign/ThirdPerson/Blueprints/BP_Player2D.BP_Player2D_C|GetProjectile_Info _as_bp_player_2d)) (* _proj_speed -1.0)) (CallFunction|VerifyAddStats (.distance (Variables|/Game/GameDesign/ThirdPerson/Blueprints/BP_Player2D.BP_Player2D_C|GetProjectile_Info _as_bp_player_2d)) (* _distance -1.0)) (.actor_ignore (Variables|/Game/GameDesign/ThirdPerson/Blueprints/BP_Player2D.BP_Player2D_C|GetProjectile_Info _as_bp_player_2d)) 0)))
  (Utilities|Array|RemoveItem _item_list _outitem)
  (Default|ItemGain (Variables|/Game/GameDesign/ThirdPerson/Blueprints/BP_Player2D.BP_Player2D_C|GetWidget_Ref _as_bp_player_2d_2))
  (Variables|Default|SetOpened? true)
  (Game|SpawnActorfromClass "/Game/GameDesign/Blueprint/PickUps/BP_PickUp_HeartContainer.BP_PickUp_HeartContainer_C" (Math|Transform|MakeTransform (Transformation|GetActorLocation) "0, 0, 0" "1.000000,1.000000,1.000000") "AlwaysSpawn" "MultiplyWithRoot" 0 0)
  (Rendering|Components|Sprite|SetSprite (Variables|Default|GetPaperSprite) "/Game/PaperAssets/Tilemap/Sprites_TileMap/tilemap_Sprite_202.tilemap_Sprite_202"))

(event EventBeginPlay
  (|CallParentFunction) ; This node is disabled and will not be called.\nDrag off pins to build functionality.
)

(event Collision|EventActorBeginOverlap
  (params (OtherActor :type Actor%20Object%20Reference))
  (|CallParentFunction OtherActor) ; This node is disabled and will not be called.\nDrag off pins to build functionality.
)

(event EventTick
  (params (DeltaSeconds :type Float%20%28single-precision%29))
  (|CallParentFunction DeltaSeconds) ; This node is disabled and will not be called.\nDrag off pins to build functionality.
)

(event EventPickUpEvent
  (params (Target :type Actor%20Object%20Reference))
  (CallFunction|Push Target 4e+01)
  (if (Utilities|Array|IsNotEmpty (Variables|/Game/GameDesign/ThirdPerson/Blueprints/BP_Player2D.BP_Player2D_C|GetItem_List (Variables|/Game/GameDesign/ThirdPerson/Blueprints/BP_ThirdPersonGameMode.BP_ThirdPersonGameMode_C|GetAs%20BP%20Player%202D (Variables|Default|GetGameModeRef))))
    (if (not (Variables|Default|GetOpened?))
      (CallFunction|Nullify))))

(fn ConstructionScript
  (|CallParentFunction))

(fn VerifyAddStats
  (params (A :type Float%20%28double-precision%29) (B :type Float%20%28double-precision%29))
  (bind _returnvalue (+ A B))
  (if (<= _returnvalue 0.0)
    (return 0.0)
    (else
      (return _returnvalue))))