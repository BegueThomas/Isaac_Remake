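; Weapon pickup that applies its AddStat modifiers to the player's 2D projectile stats, then destroys itself.
; On pickup it also stacks or adds the item in the player's ItemList and refreshes the widget.
; VerifyAddStats floors summed stats at zero, with damage sign-flipped around it to stay non-positive.
; Nullify reverses the modifiers, except damage, which it adds again without the sign flip.
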(event Custom|Add_To_Inventory
  (bind _gamemoderef (Variables|Default|GetGameModeRef))
  (bind _modify_inventory (Variables|Default|GetModify_Inventory))
  (bind _modify_inventory_2 (Variables|Default|GetModify_Inventory))
  (bind _as_bp_player_2d (Variables|/Game/GameDesign/ThirdPerson/Blueprints/BP_ThirdPersonGameMode.BP_ThirdPersonGameMode_C|GetAs%20BP%20Player%202D _gamemoderef))
  (bind _item_list (Variables|/Game/GameDesign/ThirdPerson/Blueprints/BP_Player2D.BP_Player2D_C|GetItem_List _as_bp_player_2d))
  (bind (_array_element _array_index) (Utilities|Array|ForEachLoopwithBreak _item_list :!label _label)
    (:LoopBody
      (bind _output_get (Variables|Default|SetItem_Count (.Count (Utilities|Struct|BreakST_ItemList _array_element))))
      (if (== (.Item (Utilities|Struct|BreakST_ItemList _array_element)) (.item _modify_inventory_2))
        (Variables|Default|SetItem_Collected? true)
        (Utilities|Array|SetArrayElem _item_list _array_index (Utilities|Struct|MakeST_ItemList (.item _modify_inventory_2) (+ (Variables|Default|GetItem_Count) 1.0) (.sprite _modify_inventory_2) (.object _modify_inventory_2) (.ref_addstat _modify_inventory_2)))
        (Development|PrintString (Utilities|String|ToString(Float) _output_get) true true "(R=1.000000,G=0.007398,B=0.023969,A=1.000000)")
        (goto _label Break)
        (else
          (Variables|Default|SetItem_Collected? false))))
    (:Completed
      (if (Variables|Default|GetItem_Collected?)
        _
        (else
          (Utilities|Array|Add _item_list (Utilities|Struct|MakeST_ItemList (.item _modify_inventory) 1.0 (.sprite _modify_inventory) (.object _modify_inventory) (.ref_addstat _modify_inventory)))
          (Development|PrintString "New_Item")))
      (Default|ItemGain (Variables|/Game/GameDesign/ThirdPerson/Blueprints/BP_Player2D.BP_Player2D_C|GetWidget_Ref (Variables|/Game/GameDesign/ThirdPerson/Blueprints/BP_ThirdPersonGameMode.BP_ThirdPersonGameMode_C|GetAs%20BP%20Player%202D (Variables|Default|GetGameModeRef)))))))

(event Custom|Nullify
  (bind _gamemoderef (Variables|Default|GetGameModeRef))
  (bind _add_stat (Variables|Default|GetAdd_Stat))
  (bind _as_bp_player_2d (Variables|/Game/GameDesign/ThirdPerson/Blueprints/BP_ThirdPersonGameMode.BP_ThirdPersonGameMode_C|GetAs%20BP%20Player%202D _gamemoderef))
  (Variables|/Game/GameDesign/ThirdPerson/Blueprints/BP_Player2D.BP_Player2D_C|SetProjectile_Info _as_bp_player_2d (Utilities|Struct|MakeST_Projectile (CallFunction|VerifyAddStats (.modf_fire_rate (Variables|/Game/GameDesign/ThirdPerson/Blueprints/BP_Player2D.BP_Player2D_C|GetProjectile_Info _as_bp_player_2d)) (* (.modf_fire_rate _add_stat) -1.0)) (CallFunction|VerifyAddStats (.pierce (Variables|/Game/GameDesign/ThirdPerson/Blueprints/BP_Player2D.BP_Player2D_C|GetProjectile_Info _as_bp_player_2d)) (* (.pierce _add_stat) -1.0)) (CallFunction|VerifyAddStats (.damage (Variables|/Game/GameDesign/ThirdPerson/Blueprints/BP_Player2D.BP_Player2D_C|GetProjectile_Info _as_bp_player_2d)) (.damage _add_stat)) (CallFunction|VerifyAddStats (.proj_speed (Variables|/Game/GameDesign/ThirdPerson/Blueprints/BP_Player2D.BP_Player2D_C|GetProjectile_Info _as_bp_player_2d)) (* (.proj_speed _add_stat) -1.0)) (CallFunction|VerifyAddStats (.distance (Variables|/Game/GameDesign/ThirdPerson/Blueprints/BP_Player2D.BP_Player2D_C|GetProjectile_Info _as_bp_player_2d)) (* (.distance _add_stat) -1.0)) (.actor_ignore (Variables|/Game/GameDesign/ThirdPerson/Blueprints/BP_Player2D.BP_Player2D_C|GetProjectile_Info _as_bp_player_2d)) 0)))

(event EventBeginPlay
  (|CallParentFunction)
  (Variables|Default|SetModify_Inventory (Utilities|Struct|MakeST_ItemList (.item (Variables|Default|GetModify_Inventory)) (.count (Variables|Default|GetModify_Inventory)) (.sprite (Variables|Default|GetModify_Inventory)) (.object (Variables|Default|GetModify_Inventory)) (Variables|Default|GetAdd_Stat))))

(event Collision|EventActorBeginOverlap
  (params (OtherActor :type Actor%20Object%20Reference))
  (|CallParentFunction OtherActor) ; This node is disabled and will not be called.\nDrag off pins to build functionality.
)

(event EventTick
  (params (DeltaSeconds :type Float%20%28single-precision%29))
  (|CallParentFunction DeltaSeconds) ; This node is disabled and will not be called.\nDrag off pins to build functionality.
)

(event EventPickUpEvent
  (params (Target :type Actor%20Object%20Reference))
  (bind _gamemoderef (Variables|Default|GetGameModeRef))
  (bind _add_stat (Variables|Default|GetAdd_Stat))
  (bind _as_bp_player_2d (Variables|/Game/GameDesign/ThirdPerson/Blueprints/BP_ThirdPersonGameMode.BP_ThirdPersonGameMode_C|GetAs%20BP%20Player%202D _gamemoderef))
  (Variables|/Game/GameDesign/ThirdPerson/Blueprints/BP_Player2D.BP_Player2D_C|SetProjectile_Info _as_bp_player_2d (Utilities|Struct|MakeST_Projectile (CallFunction|VerifyAddStats (.modf_fire_rate (Variables|/Game/GameDesign/ThirdPerson/Blueprints/BP_Player2D.BP_Player2D_C|GetProjectile_Info _as_bp_player_2d)) (.modf_fire_rate _add_stat)) (CallFunction|VerifyAddStats (.pierce (Variables|/Game/GameDesign/ThirdPerson/Blueprints/BP_Player2D.BP_Player2D_C|GetProjectile_Info _as_bp_player_2d)) (.pierce _add_stat)) (* (CallFunction|VerifyAddStats (* (.damage (Variables|/Game/GameDesign/ThirdPerson/Blueprints/BP_Player2D.BP_Player2D_C|GetProjectile_Info _as_bp_player_2d)) -1.0) (* (.damage _add_stat) -1.0)) -1.0) (CallFunction|VerifyAddStats (.proj_speed (Variables|/Game/GameDesign/ThirdPerson/Blueprints/BP_Player2D.BP_Player2D_C|GetProjectile_Info _as_bp_player_2d)) (.proj_speed _add_stat)) (CallFunction|VerifyAddStats (.distance (Variables|/Game/GameDesign/ThirdPerson/Blueprints/BP_Player2D.BP_Player2D_C|GetProjectile_Info _as_bp_player_2d)) (.distance _add_stat)) (.actor_ignore (Variables|/Game/GameDesign/ThirdPerson/Blueprints/BP_Player2D.BP_Player2D_C|GetProjectile_Info _as_bp_player_2d)) 0))
  (CallFunction|AddtoInventory)
  (Actor|DestroyActor))

(fn ConstructionScript
  (|CallParentFunction))

(fn VerifyAddStats
  (params (A :type Float%20%28double-precision%29) (B :type Float%20%28double-precision%29))
  (bind _returnvalue (+ A B))
  (if (<= _returnvalue 0.0)
    (return 0.0)
    (else
      (return _returnvalue))))